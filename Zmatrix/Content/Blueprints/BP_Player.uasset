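; BP_Player is the player actor, which moves in the Y-Z plane and fires projectiles.
; MoveRight and MoveUp axes set horizontal and vertical speeds, which Tick applies as a swept per-frame offset, not scaled by delta time.
; FirePrimary fires immediately and starts a looping timer that spawns BP_ProjectilePlayerBase at the spawn point.
; Release clears the timer and resets the DoOnce gate.
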(event Custom|FirePressed
  (Utilities|FlowControl|DoOnce false
    (:Completed
      (CallFunction|Fire)
      (Utilities|Time|SetTimerbyFunctionName 0 "Fire" 0.2 true))))

(event Custom|Fire
  (Game|SpawnActorfromClass "/Game/Blueprints/BP_ProjectilePlayerBase.BP_ProjectilePlayerBase_C" (Transformation|GetWorldTransform (Variables|Default|GetProjecttileSpawnPoint)) "Undefined" 0 "(R=0.000000,G=0.000000,B=0.000000,A=0.000000)" 0))

(event Custom|FireReleased
  (Utilities|Time|ClearTimerbyFunctionName 0 "Fire")
  (Utilities|FlowControl|DoOnce false) ; enters at Reset
)

(event EventTick
  (params (DeltaSeconds :type Float%20%28single-precision%29))
  (Variables|Default|SetDeltaSeconds DeltaSeconds)
  (Transformation|SetActorLocation (+ (Transformation|GetActorLocation) (Math|Vector|MakeVector 0.0 (Variables|Default|GetHozSpeed) (Variables|Default|GetVertSpeed))) true false))

(event Input|ActionEvents|InputActionFirePrimary
  (params (Key :type Key%20Structure))
  (:Pressed
    (CallFunction|FirePressed))
  (:Released
    (CallFunction|FireReleased)))

(event Input|AxisEvents|InputAxisMoveUp
  (params (AxisValue :type Float%20%28single-precision%29))
  (Variables|Default|SetVertSpeed (* AxisValue (Variables|Default|GetMovementSpeed))))

(event Input|AxisEvents|InputAxisMoveRight
  (params (AxisValue :type Float%20%28single-precision%29))
  (Variables|Default|SetHozSpeed (* AxisValue (Variables|Default|GetMovementSpeed))))

(fn ConstructionScript)